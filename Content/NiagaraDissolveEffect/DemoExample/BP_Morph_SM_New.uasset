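; Niagara demo actor that plays a looping dissolve morph between two static mesh actors selected in the level.
; The construction script assigns both meshes and materials and creates the particle material instance.
; BeginPlay spawns the Niagara system on the first mesh and feeds it both mesh components.
; Two staggered timelines drive dissolve amounts in a Material Parameter Collection, then the effect is destroyed, reset and respawned.
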(event `self.ReceiveBeginPlay`
  (bind _staticmeshcomponent (`StaticMeshActor.StaticMeshComponent` (`self.Mesh`)))
  (bind _returnvalue (`NiagaraFunctionLibrary.SpawnSystemAttached` "/Game/NiagaraDissolveEffect/Niagara/P_Morph_SM_New.P_Morph_SM_New" _staticmeshcomponent "None" (0.0 0.0 0.0) (struct) "KeepRelativeOffset" :!label _label))
  (`NiagaraComponent.SetVariableMaterial` _returnvalue "Material Interface" (`self.MI`))
  ;[1 1 1] Morph Anim Setting
  (`NiagaraFunctionLibrary.OverrideSystemUserVariableStaticMeshComponent` _returnvalue "Static Mesh0" _staticmeshcomponent)
  (`NiagaraFunctionLibrary.OverrideSystemUserVariableStaticMeshComponent` _returnvalue "Static Mesh1" (`StaticMeshActor.StaticMeshComponent` (`self.Mesh_1`)))
  (`TimelineComponent.SetPlayRate` (`self.Timeline_0`) (`self.DissolveAnimRate`))
  (`|ExecutionSequence`
    (:`then_0`
      (bind (_direction _newtrack_0) (`Timeline|Timeline_0` :!via `PlayFromStart`)
        (:`Update`
          (`KismetMaterialLibrary.SetScalarParameterValue` "/Game/NiagaraDissolveEffect/DemoRoom/StaticMeshExample/Materials/Morph/MPC_Morph_SM.MPC_Morph_SM" "Amount" _newtrack_0))))
    (:`then_1`
      (`KismetSystemLibrary.Delay` 2.0)
      ;[1 1 1] Morph Anim Setting
      (`TimelineComponent.SetPlayRate` (`self.Timeline_1`) (`self.DissolveAnimRate1`))
      (bind (_direction_2 _newtrack_0_2) (`Timeline|Timeline_1` :!via `PlayFromStart`)
        (:`Update`
          (`KismetMaterialLibrary.SetScalarParameterValue` "/Game/NiagaraDissolveEffect/DemoRoom/StaticMeshExample/Materials/Morph/MPC_Morph_SM.MPC_Morph_SM" "Amount1" (- 1.0 _newtrack_0_2)))
        (:`Finished`
          ;[1 1 1] Reset
          (`ActorComponent.K2_DestroyComponent` _returnvalue)
          (`KismetSystemLibrary.Delay` 1.0)
          (`KismetMaterialLibrary.SetScalarParameterValue` "/Game/NiagaraDissolveEffect/DemoRoom/StaticMeshExample/Materials/Morph/MPC_Morph_SM.MPC_Morph_SM" "Amount1")
          (`KismetMaterialLibrary.SetScalarParameterValue` "/Game/NiagaraDissolveEffect/DemoRoom/StaticMeshExample/Materials/Morph/MPC_Morph_SM.MPC_Morph_SM" "Amount" 1.0)
          (goto _label))))))

(fn `UserConstructionScript`
  (bind _staticmeshcomponent (`StaticMeshActor.StaticMeshComponent` (`self.Mesh_1`)))
  (bind _staticmeshcomponent_2 (`StaticMeshActor.StaticMeshComponent` (`self.Mesh`)))
  (`StaticMeshComponent.SetStaticMesh` _staticmeshcomponent_2 (`self.Set Static Mesh`))
  (`PrimitiveComponent.SetMaterial` _staticmeshcomponent_2 0 (`self.Mesh Material`))
  (`StaticMeshComponent.SetStaticMesh` _staticmeshcomponent (`self.Set Static Mesh_1`))
  (`PrimitiveComponent.SetMaterial` _staticmeshcomponent 0 (`self.Mesh Material_1`))
  (bind _returnvalue (`KismetMaterialLibrary.CreateDynamicMaterialInstance` (`self.M_Niagara`)))
  (set `self.MI` _returnvalue))