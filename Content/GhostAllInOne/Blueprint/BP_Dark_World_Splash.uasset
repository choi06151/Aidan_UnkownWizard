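; Blueprint that toggles a Dark World splash effect around the player character when F is pressed.
; Each press writes the character mesh location into the MP_Dark_World parameter collection, then alternates playing and reversing the Splash timeline.
; The timeline drives the collection's DW Radius parameter.
; The forward press also enables DarkWorld after a short delay; reversing never disables it.
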(event `Key|F`
  (params (Key :type "Key Structure"))
  ;[1 1 1] Replace if need
  (:`Pressed`
    ;[1 1 1] Activation Code
    (`KismetMaterialLibrary.SetVectorParameterValue` "/Game/GhostAllInOne/Material_Function/MP_Dark_World.MP_Dark_World" "DW Player State" (`KismetMathLibrary.Conv_VectorToLinearColor` (`SceneComponent.K2_GetComponentLocation` (`Character.Mesh` (`GameplayStatics.GetPlayerCharacter` 0)))))
    (`/Engine/EditorBlueprintResources/StandardMacros.FlipFlop`
      (:`A`
        (`|ExecutionSequence`
          (:`then_0`
            (bind (_direction _newtrack_0) (`Timeline|Splash` :!label _label)
              (:`Update`
                (`KismetMaterialLibrary.SetScalarParameterValue` "/Game/GhostAllInOne/Material_Function/MP_Dark_World.MP_Dark_World" "DW Radius" _newtrack_0))))
          (:`then_1`
            (`KismetSystemLibrary.Delay` 1.0)
            (set `PostProcessComponent.bEnabled` true (`self.Dark_World`)))))
      (:`B`
        (goto _label :!via `Reverse`)))))

(fn `UserConstructionScript`)