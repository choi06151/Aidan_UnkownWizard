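; DoReMi_Player_BP plays musical pickup sounds in sequence, so successive pickups step through a series such as a scale.
; PlayPickUpSound plays the current entry of the SoundsToPlay array at a given location, then calls SetNextIndex.
; SetNextIndex advances CurrentIndex and wraps to the first sound after the last one.
; The event graph and construction script are empty, so playback depends on external callers.
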(fn `Play Pick up sound`
  (params (Location :type "Vector Structure"))
  (`GameplayStatics.PlaySoundAtLocation` (`|GetArrayItem` (`self.Sounds to Play`) (`self.Current Index`)) Location (struct) 1.0 1.0 0.0 null null null)
  (`self.Set Next Index`))

(fn `Set Next Index`
  (set `self.Current Index` (`KismetMathLibrary.SelectInt` (+ (`self.Current Index`) 1) 0 (< (`self.Current Index`) (`KismetArrayLibrary.Array_LastIndex` (`self.Sounds to Play`))))))

(fn `UserConstructionScript`)