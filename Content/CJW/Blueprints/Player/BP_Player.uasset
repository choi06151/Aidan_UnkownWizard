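; VR hand-tracked player for a music-themed combat game, holding HP, score, bullet upgrades and five collectible note slots.
; Tick aims a confidence-gated spline laser for widget interaction and tracks palm direction, fists and hand distance to drive BP_Staff's states and skill selection.
; Staff-reported notes fill slots, which four skills spend: slow, temporary invulnerability, staff attack and paralysis shot.
; Gesture recognition only prints; debug keys record/delete gestures and spawn test notes.
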(event `Key|B`
  (params (Key :type "Key Structure")))

(event `Key|Zero`
  (params (Key :type "Key Structure")))

(event `self.ReceiveBeginPlay`
  (`|ExecutionSequence`
    (:`then_0`
      ;[1 1 1] 헤드셋을 쓰고 있다면
      (if (`HeadMountedDisplayFunctionLibrary.IsHeadMountedDisplayEnabled`)
        ;[1 1 1] 패스스루 모드 시작
        (`OculusXRFunctionLibrary.IsPassthroughRecommended`)
        ;[1 1 1] 위치조정
        (`HeadMountedDisplayFunctionLibrary.SetTrackingOrigin` "Eye")))
    (:`then_1`
      (add `/Game/CJW/Blueprints/Player/Hand/BPC_PlayerRightHand.OnGestureRecognisedRight` (`self.BPC_PlayerRightHand`) (delegate `GestureRecognised`))
      (add `/Game/CJW/Blueprints/Player/Hand/BPC_PlayerLeftHand.OnGestureRecognisedLeft` (`self.BPC_PlayerLeftHand`) (delegate `GestureRecognised`))
      (add `self.WantUseSkill` (delegate `UseSkill`))
      (add `self.GetNoteInfo` (delegate `GetNoteInfoFromStaff`)))
    (:`then_2`
      (`self.StartSetting`))))

(event `Key|E`
  (params (Key :type "Key Structure"))
  (bind (_once _twice _triple _quad _fifth) (break `/Game/CJW/Blueprints/Skill/S_Note` (`self.NoteForSkill`)))
  (:`Pressed`
    (`KismetSystemLibrary.PrintString` (`KismetStringLibrary.Conv_BoolToString` _once))
    (`KismetSystemLibrary.PrintString` (`KismetStringLibrary.Conv_BoolToString` _twice))
    (`KismetSystemLibrary.PrintString` (`KismetStringLibrary.Conv_BoolToString` _triple))
    (`KismetSystemLibrary.PrintString` (`KismetStringLibrary.Conv_BoolToString` _quad))
    (`KismetSystemLibrary.PrintString` (`KismetStringLibrary.Conv_BoolToString` _fifth))))

(event `Key|V`
  (params (Key :type "Key Structure"))
  ;[1 1 1] 제스쳐 녹음 밑 삭제
  (:`Pressed`
    (`/Game/CJW/Blueprints/Player/Hand/BPC_PlayerLeftHand.RecordGesture` (`self.BPC_PlayerLeftHand`) (`self.GestureName`))
    (`KismetSystemLibrary.PrintString` "정상 녹음 완료 ")))

(event `GetNoteInfoFromStaff` :!signature `self.GetNoteInfo`
  (params (NoteInfo :type "/Game/CJW/Blueprints/Skill/E_NoteType Enum" :default "NewEnumerator0"))
  (`self.GetNote` NoteInfo))

(event `Key|C`
  (params (Key :type "Key Structure"))
  ;[1 1 1] 제스쳐 녹음 밑 삭제
  (:`Pressed`
    (`/Game/CJW/Blueprints/Player/Hand/BPC_PlayerRightHand.RecordGesture` (`self.BPC_PlayerRightHand`) (`self.GestureName`))
    (`KismetSystemLibrary.PrintString` "정상 녹음 완료 ")))

(event `Press`
  ;[1 1 1] 입력설정 , 마우스클릭을 대신 하게 적용
  (`WidgetInteractionComponent.PressPointerKey` (`self.WidgetInteraction`) "LeftMouseButton"))

(event `UseSkill` :!signature `self.WantUseSkill`
  (params (NewParam :type "/Game/CJW/Blueprints/Skill/E_SKills Enum" :default "NewEnumerator0"))
  ;[1 1 1] 스킬 실행
  (switch `/Game/CJW/Blueprints/Skill/E_SKills` NewParam
    (:`NewEnumerator0`
      (`self.SlowSkill`))
    (:`NewEnumerator1`
      (`self.SuperArmor`))
    (:`NewEnumerator2`
      (`self.StaffSkill`))
    (:`NewEnumerator3`
      (`self.ParalyzationAttack`))))

(event `Key|B`
  (params (Key :type "Key Structure"))
  ;[1 1 1] 제스쳐 녹음 밑 삭제
  (:`Pressed`
    (`/Game/CJW/Blueprints/Player/Hand/BPC_PlayerRightHand.DeleteGesture` (`self.BPC_PlayerRightHand`) (`self.GestureName`))
    (`KismetSystemLibrary.PrintString` "정상 삭제 완료 ")))

(event `GestureRecognised`
  (params (GestureName :type String))
  ;[1 1 1] 제스쳐 실행
  (switch `string` GestureName
    (:`V`
      (`KismetSystemLibrary.PrintString` "vivi정상 출력"))
    (:`Shot`
      (`KismetSystemLibrary.PrintString` "shot정상 출력"))
    (:`OK`
      (`KismetSystemLibrary.PrintString` "OK정상 출력"))))

(event `Released`
  ;[1 1 1] 입력설정 , 마우스클릭을 대신 하게 적용
  (`WidgetInteractionComponent.ReleasePointerKey` (`self.WidgetInteraction`) "LeftMouseButton"))

(event `Key|A`
  (params (Key :type "Key Structure"))
  ;[1 1 1] test를 위한 노드 생성
  (:`Pressed`
    (`|SpawnActorFromClass` "/Game/CJW/Blueprints/Skill/BP_NodeForTest.BP_NodeForTest_C" (`KismetMathLibrary.MakeTransform` (+ (`self.K2_GetActorLocation` self) (* (`self.GetActorForwardVector` self) 1000.0))) "Undefined" "MultiplyWithRoot" null null)))

(event `self.ReceiveTick`
  (params (DeltaSeconds :type "Float (single-precision)"))
  (bind _returnvalue (`self.GetTransform`))
  (bind (_returnvalue_location _returnvalue_rotation) (`KismetMathLibrary.BreakTransform` (`OculusXRInputFunctionLibrary.GetPointerPose` "HandRight")))
  (bind _output (`self.DetectCanUseStaffSkillHand`))
  (bind _blefthandgrab (`/Game/CJW/Blueprints/Player/Hand/BPC_PlayerLeftHand.bLeftHandGrab` (`self.BPC_PlayerLeftHand`)))
  (bind _brighthandgrab (`/Game/CJW/Blueprints/Player/Hand/BPC_PlayerRightHand.bRightHandGrab` (`self.BPC_PlayerRightHand`)))
  (bind (_bblockinghit _binitialoverlap _time _distance _location) (`GameplayStatics.BreakHitResult` (`WidgetInteractionComponent.GetLastHitResult` (`self.WidgetInteraction`))))
  (bind _returnvalue_2 (`KismetMathLibrary.Vector_Distance` (`SceneComponent.K2_GetComponentLocation` (`self.MotionControllerRight`)) (`SceneComponent.K2_GetComponentLocation` (`self.MotionControllerLeft`))))
  ;[1 1 1] 레이저 신용확인 , 항상 레이저가 나가는걸 방지
  (`|ExecutionSequence`
    (:`then_0`
      (switch `EOculusXRTrackingConfidence` (`OculusXRInputFunctionLibrary.GetTrackingConfidence` "HandRight")
        (:`Low`
          (`self.CollapseSpline`))
        (:`High`
          ;[1 1 1] 신용도가 높더라도 유효성검사
          (if (`OculusXRInputFunctionLibrary.IsPointerPoseValid` "HandRight")
            ;[1 1 1] 레이져 사출
            (`SceneComponent.K2_SetWorldLocationAndRotation` (`self.Spline`) (`KismetMathLibrary.TransformLocation` _returnvalue _returnvalue_location) (`KismetMathLibrary.TransformRotation` _returnvalue _returnvalue_rotation) false false)
            (`SceneComponent.K2_SetWorldLocationAndRotation` (`self.WidgetInteraction`) (`KismetMathLibrary.TransformLocation` _returnvalue _returnvalue_location) (`KismetMathLibrary.TransformRotation` _returnvalue _returnvalue_rotation) false false)
            (if _bblockinghit
              ;[1 1 1] 사출하여 피격된 위치로 레이져 이동
              (`SplineComponent.SetLocationAtSplinePoint` (`self.Spline`) 1 _location "World" true)
              (`self.UpdateSplineMesh`)
              (else
                (`self.CollapseSpline`)))
            (else
              (`self.CollapseSpline`))))))
    (:`then_1`
      (`self.DetectHandDirection`))
    (:`then_2`
      ;[1 1 1] 스킬 매커니즘 설명1.두 손을 붙였을때 생성 가능 2. 왼,우 주먹 그리고 0~90거리 까지 벌리기 3. 일정 거리가 넘으면 완전 펴짐
      ;;[1 1 1] 조건 1.양손의 손바닥위치가 반대, 양손의 손바닥 거리 20미만, 양손이 주먹 . 양손의 거리가 멀때 오선지가 생기는걸 방지
      (if (and _blefthandgrab _brighthandgrab (< _returnvalue_2 20.0) _output)
        (set `self.bStaffPossible` true)))
    (:`then_3`
      (if (`self.bStaffSkillSelectPossible`)
        _
        (elif (and _blefthandgrab _brighthandgrab (> _returnvalue_2 0.0) (`self.bStaffPossible`) _output)
          ;;[1 1 1] 0~ 90 까지는 공격 흡수
          (set `/Game/CJW/Blueprints/UI/Actor/BP_Staff.CurrentState` "NewEnumerator1" (`self.Staff`))
          ;;[1 1 1] 90부터는 스킬사용,오른손만 놓으면 스킬 사용을 위한 오선지 세팅 , 오른손을 놓지 않고  일정 거리 넘으면 파괴
          (if (> _returnvalue_2 60.0)
            (set `self.bStaffSkillSelectPossible` true))
          (else
            ;;[1 1 1] 중복 적용 방지 검사
            (if (and (`|EnumInequality` (`/Game/CJW/Blueprints/UI/Actor/BP_Staff.CurrentState` (`self.Staff`)) "NewEnumerator0") (not (`/Game/CJW/Blueprints/UI/Actor/BP_Staff.bAttackSKillMode` (`self.Staff`))))
              (set `/Game/CJW/Blueprints/UI/Actor/BP_Staff.CurrentState` "NewEnumerator0" (`self.Staff`))
              (set `self.bStaffPossible` false)
              (`/Game/CJW/Blueprints/UI/Widget/WBP_Staff.InitializeInfo` (`/Game/CJW/Blueprints/UI/Actor/BP_Staff.As WBP Staff` (`self.Staff`))))))))
    (:`then_4`
      (if (`self.bSkillSelectModeOn`)
        ;;[1 1 1] 스킬 선택모드
        (if (`/Game/CJW/Blueprints/Player/Hand/BPC_PlayerLeftHand.bLeftHandGrab` (`self.BPC_PlayerLeftHand`))
          (set `/Game/CJW/Blueprints/UI/Actor/BP_Staff.CurrentState` "NewEnumerator2" (`self.Staff`))
          (else
            (set `self.bStaffPossible` false)
            (set `self.bStaffSkillSelectPossible` false)
            (set `self.bSkillSelectModeOn` false)
            (`/Game/CJW/Blueprints/UI/Widget/WBP_Staff.Playercheckuse` (`/Game/CJW/Blueprints/UI/Actor/BP_Staff.As WBP Staff` (`self.Staff`)))))
        (else
          ;;[1 1 1] 조건 3 손바닥 위치 상관 x, 왼손은 주먹 ,오른손 엄지를  폈을때
          (if (and (`self.bStaffSkillSelectPossible`) (`/Game/CJW/Blueprints/Player/Hand/BPC_PlayerLeftHand.bLeftHandGrab` (`self.BPC_PlayerLeftHand`)) (not (`/Game/CJW/Blueprints/Player/Hand/BPC_PlayerRightHand.bRightHandGrab` (`self.BPC_PlayerRightHand`))))
            ;;[1 1 1] 스킬 선택모드가능
            (set `self.bSkillSelectModeOn` true)))))))

(event `self.HitBox.OnComponentBeginOverlap`
  (params (OverlappedComponent :type "PrimitiveComponent Object Reference") (OtherActor :type "Actor Object Reference") (OtherComp :type "PrimitiveComponent Object Reference") (OtherBodyIndex :type Integer) (bFromSweep :type Boolean) (SweepResult :type "HitResult Structure (by ref)"))
  ;[1 1 1] 임의생성한 노트를 얻으면 랜덤으로 노트를 채우고, 해당 오버랩한 물체를 부신다
)

(event `WantSkillUse`
  (`/Game/CJW/Blueprints/UI/Widget/WBP_Staff.Playercheckuse` (`/Game/CJW/Blueprints/UI/Actor/BP_Staff.StaffWidget` (`self.Staff`))))

(event `GetHPItem`
  ;[1 1 1] 아이템 관련노드
  ;;[1 1 1] Get함수들
  (`self.HPSet` 20.0 true))

(event `BasicAttack`
  (bind _camera (`self.Camera`))
  ;[1 1 1] 스킬 관련 노드
  ;;[1 1 1] 기본 평타
  (for _ (range (+ (`self.CurrentSpawnBulletCount`) 1))
    (`|SpawnActorFromClass` "/Game/CJW/Blueprints/Bullet/BP_PlayerBullet.BP_PlayerBullet_C" (`KismetMathLibrary.MakeTransform` (`SceneComponent.K2_GetComponentLocation` _camera) (`KismetMathLibrary.Conv_VectorToRotator` (`KismetMathLibrary.Conv_RotatorToVector` (`SceneComponent.K2_GetComponentRotation` _camera))) (`self.BulletActtackScale`)) "Undefined" "MultiplyWithRoot" null (`self.BulletAttackSpeed`) (`self.BulletAttackDamage`) null)))

(event `GetScoreItem`
  ;[1 1 1] 아이템 관련노드
  ;;[1 1 1] Get함수들
  (`self.ScoreSet` 100.0 true))

(event `InputAction|RightMiddle`
  (params (Key :type "Key Structure"))
  ;[1 1 1] 중지를눌럿을때 메뉴가 뜨게 하기
)

(event `ParalyzationAttack`
  (bind _camera (`self.Camera`))
  ;[1 1 1] 스킬 관련 노드
  ;;[1 1 1] 뮤트
  (bind _bskillcanuse (`self.CheckForUseSkill` "NewEnumerator3" (`self.NoteForSkill`)))
  (if _bskillcanuse
    (`|SpawnActorFromClass` "/Game/CJW/Blueprints/Bullet/BP_paralyzation.BP_paralyzation_C" (`KismetMathLibrary.MakeTransform` (`SceneComponent.K2_GetComponentLocation` _camera) (`KismetMathLibrary.Conv_VectorToRotator` (`KismetMathLibrary.Conv_RotatorToVector` (`SceneComponent.K2_GetComponentRotation` _camera))) (`self.BulletActtackScale`)) "Undefined" "MultiplyWithRoot" null (`self.BulletAttackSpeed`) (`self.BulletAttackDamage`) null)
    (`/Game/CJW/Blueprints/UI/Widget/WBP_Staff.UpdatePlayerNoteInfo` (`/Game/CJW/Blueprints/UI/Actor/BP_Staff.As WBP Staff` (`self.Staff`)) (`self.NoteForSkill`))))

(event `GetBulletSpeedItem`
  ;[1 1 1] 아이템 관련노드
  ;;[1 1 1] 총알 속도 빨라지는 노드
  (set `self.BulletAttackSpeed` (+ (`self.BulletAttackSpeed`) 100.0)))

(event `InputAction|LeftMiddel`
  (params (Key :type "Key Structure"))
  (bind _camera (`self.Camera`))
  (bind _returnvalue (`SceneComponent.K2_GetComponentLocation` _camera))
  (bind _returnvalue_2 (+ _returnvalue (* (`SceneComponent.GetForwardVector` _camera) 4000.0)))
  ;[1 1 1] 메뉴 관련
  (:`Pressed`
    (`|SpawnActorFromClass` "/Game/CJW/Blueprints/Skill/BP_NodeForTest.BP_NodeForTest_C" (`KismetMathLibrary.MakeTransform` _returnvalue_2 (`KismetMathLibrary.FindLookAtRotation` _returnvalue_2 _returnvalue)) "Undefined" "MultiplyWithRoot" null null)))

(event `GetBulletAmountItem`
  ;[1 1 1] 아이템 관련노드
  ;;[1 1 1] 총알 개수 많아지는 노드
  (`/Engine/EditorBlueprintResources/StandardMacros.IncrementInt` (`self.CurrentSpawnBulletCount`)))

(event `InputAction|RightIndexRing`
  (params (Key :type "Key Structure"))
  ;[1 1 1] 메뉴 관련
  (:`Pressed`
    (`self.Press`))
  (:`Released`
    (`self.Released`)))

(event `SlowSkill`
  ;[1 1 1] 스킬 관련 노드
  ;;[1 1 1] 리타르단도 (게임모드, 혹은 게임스테이트에 느려지게 하는 노드 만들어야함
  (bind _bskillcanuse (`self.CheckForUseSkill` "NewEnumerator0" (`self.NoteForSkill`)))
  (if _bskillcanuse
    (bind _asvrgame_mode (cast `/Game/VRTemplate/Blueprints/VRGameMode` (`GameplayStatics.GetGameMode`)))
    (`/Game/VRTemplate/Blueprints/VRGameMode.StartSLow` _asvrgame_mode)
    (`/Game/CJW/Blueprints/UI/Widget/WBP_Staff.UpdatePlayerNoteInfo` (`/Game/CJW/Blueprints/UI/Actor/BP_Staff.As WBP Staff` (`self.Staff`)) (`self.NoteForSkill`))))

(event `GetBulletSizeItem`
  ;[1 1 1] 아이템 관련노드
  ;;[1 1 1] 총알 크기 커지는 노드
  (set `self.BulletActtackScale` (+ (`self.BulletActtackScale`) (1.0 1.0 1.0))))

(event `GetBulletCooltimeItem`
  ;[1 1 1] 아이템 관련노드
  (set `self.BulletCoolTIme` (- (`self.BulletCoolTIme`) 10.0)))

(event `StaffSkill`
  ;[1 1 1] 스킬 관련 노드
  ;;[1 1 1] 크레센도 (오선지 쓸기)
  (if true
    (bind _bskillcanuse (`self.CheckForUseSkill` "NewEnumerator2" (`self.NoteForSkill`)))
    (if _bskillcanuse
      (`/Game/CJW/Blueprints/UI/Actor/BP_Staff.StartStaffAttack` (`self.Staff`))
      (`/Game/CJW/Blueprints/UI/Widget/WBP_Staff.UpdatePlayerNoteInfo` (`/Game/CJW/Blueprints/UI/Actor/BP_Staff.As WBP Staff` (`self.Staff`)) (`self.NoteForSkill`)))))

(event `SuperArmor`
  ;[1 1 1] 스킬 관련 노드
  ;;[1 1 1] 포르티시모
  (bind _bskillcanuse (`self.CheckForUseSkill` "NewEnumerator1" (`self.NoteForSkill`)))
  (if _bskillcanuse
    (`PrimitiveComponent.SetCollisionEnabled` (`self.HitBox`) "NoCollision")
    (`KismetSystemLibrary.Delay` 10.0)
    (`PrimitiveComponent.SetCollisionEnabled` (`self.HitBox`) "QueryAndPhysics")
    (`/Game/CJW/Blueprints/UI/Widget/WBP_Staff.UpdatePlayerNoteInfo` (`/Game/CJW/Blueprints/UI/Actor/BP_Staff.StaffWidget` (`self.Staff`)) (`self.NoteForSkill`))))

(fn `CheckForUseSkill`
  (params (SkillType :type "/Game/CJW/Blueprints/Skill/E_SKills Enum" :default "NewEnumerator0") (PlayerNote :type "/Game/CJW/Blueprints/Skill/S_Note Structure"))
  (returns (bSKillCanUSe :type Boolean))
  (bind (_once _twice _triple _quad _fifth) (break `/Game/CJW/Blueprints/Skill/S_Note` PlayerNote))
  (switch `/Game/CJW/Blueprints/Skill/E_SKills` SkillType
    (:`NewEnumerator0`
      ;[1 1 1] 리타르단도 (1,3,5 참)
      (if (and (== _once true) (== _triple true) (== _fifth true))
        (set `self.NoteForSkill` (make `/Game/CJW/Blueprints/Skill/S_Note` false _twice false _quad))
        (`/Game/CJW/Blueprints/UI/Widget/WBP_Staff.InitializeInfo` (`/Game/CJW/Blueprints/UI/Actor/BP_Staff.As WBP Staff` (`self.Staff`)))
        (return true)
        (else
          (return false))))
    (:`NewEnumerator1`
      ;[1 1 1] 포르티시모(2,3,5 참)
      (if (and (== _twice true) (== _triple true) (== _fifth true))
        (set `self.NoteForSkill` (make `/Game/CJW/Blueprints/Skill/S_Note` _once false false _quad))
        (`/Game/CJW/Blueprints/UI/Widget/WBP_Staff.InitializeInfo` (`/Game/CJW/Blueprints/UI/Actor/BP_Staff.As WBP Staff` (`self.Staff`)))
        (return true)
        (else
          (return false))))
    (:`NewEnumerator2`
      ;[1 1 1] 크레센도(1,2,3,4,5참)
      (if (and (== _once true) (== _twice true) (== _triple true) (== _quad true) (== _fifth true))
        (set `self.NoteForSkill` (make `/Game/CJW/Blueprints/Skill/S_Note` false))
        (`/Game/CJW/Blueprints/UI/Widget/WBP_Staff.InitializeInfo` (`/Game/CJW/Blueprints/UI/Actor/BP_Staff.As WBP Staff` (`self.Staff`)))
        (return true)
        (else
          (return false))))
    (:`NewEnumerator3`
      ;[1 1 1] 뮤트(1,5 참)
      (if (and (== _once true) (== _fifth true))
        (set `self.NoteForSkill` (make `/Game/CJW/Blueprints/Skill/S_Note` false _twice _triple _quad))
        (`/Game/CJW/Blueprints/UI/Widget/WBP_Staff.InitializeInfo` (`/Game/CJW/Blueprints/UI/Actor/BP_Staff.As WBP Staff` (`self.Staff`)))
        (return true)
        (else
          (return false))))))

(fn `CollapseSpline`
  ;[1 1 1] 선의 시작을 0 , 끝을 1의  포인트라 했을때 선형보간으로 부드럽게 레이저가 나가는 형식, 0과 1로 나눠져있을때  0을 1로 바꾸어 레이져를 없앤다
  (`SplineComponent.SetLocationAtSplinePoint` (`self.Spline`) 1 (`SplineComponent.GetLocationAtSplinePoint` (`self.Spline`) 0 "World") "World" true)
  (`self.UpdateSplineMesh`))

(fn `DetectCanUseStaffSkillHand`
  (returns (Output :type Boolean))
  (return (or (and (== (`self.bRightL`) true) (== (`self.bRightR`) true)) (and (== (`self.bUpperL`) false) (== (`self.bUpperR`) true)) (and (== (`self.bUpperL`) true) (== (`self.bUpperR`) false)))))

(fn `DetectHandDirection`
  (bind _returnvalue (`KismetMathLibrary.Dot_VectorVector` (`SceneComponent.GetUpVector` (`self.BPC_PlayerRightHand`)) (0.0 0.0 -1.0)))
  (bind _returnvalue_2 (`KismetMathLibrary.Dot_VectorVector` (`SceneComponent.GetUpVector` (`self.BPC_PlayerLeftHand`)) (0.0 0.0 1.0)))
  (`|ExecutionSequence`
    (:`then_0`
      ;[1 1 1] 왼쪽 손바닥이 위인가 ?
      (if (> (`KismetMathLibrary.Dot_VectorVector` (`SceneComponent.GetUpVector` (`self.BPC_PlayerLeftHand`)) (0.0 0.0 1.0)) 0.5)
        (set `self.bUpperL` true)
        (else
          (set `self.bUpperL` false))))
    (:`then_1`
      ;[1 1 1] 오른쪽 손바닥이 위인가 ?
      (if (> (`KismetMathLibrary.Dot_VectorVector` (`SceneComponent.GetUpVector` (`self.BPC_PlayerRightHand`)) (0.0 0.0 -1.0)) 0.5)
        (set `self.bUpperR` true)
        (else
          (set `self.bUpperR` false))))
    (:`then_2`
      ;[1 1 1] 왼쪽 손바닥이  옆을 바라보고 있나 ?
      (if (== (<= _returnvalue_2 0.5) (>= _returnvalue_2 -0.5))
        (set `self.bRightL` true)
        (else
          (set `self.bRightL` false))))
    (:`then_3`
      ;[1 1 1] 오른쪽 손바닥이 오른쪽을 바라보고 있나 ?
      (if (== (<= _returnvalue 0.5) (>= _returnvalue -0.5))
        (set `self.bRightR` true)
        (else
          (set `self.bRightR` false))))))

(fn `GetNote`
  (params (GetNoteType :type "/Game/CJW/Blueprints/Skill/E_NoteType Enum" :default "NewEnumerator0"))
  (bind (_once _twice _triple _quad) (break `/Game/CJW/Blueprints/Skill/S_Note` (`self.NoteForSkill`)))
  (bind (_once_2 _twice_2 _triple_2 _quad_2 _fifth) (break `/Game/CJW/Blueprints/Skill/S_Note` (`self.NoteForSkill`)))
  (bind (_once_3 _twice_3 _triple_3 _quad_3 _fifth_2) (break `/Game/CJW/Blueprints/Skill/S_Note` (`self.NoteForSkill`)))
  (bind (_once_4 _twice_4 _triple_4 _quad_4 _fifth_3) (break `/Game/CJW/Blueprints/Skill/S_Note` (`self.NoteForSkill`)))
  (bind (_once_5 _twice_5 _triple_5 _quad_5 _fifth_4) (break `/Game/CJW/Blueprints/Skill/S_Note` (`self.NoteForSkill`)))
  (switch `/Game/CJW/Blueprints/Skill/E_NoteType` GetNoteType
    (:`NewEnumerator1`
      ;[1 1 1] 나머지는 그대로 가져가고 얻는정보만 변환
      (set `self.NoteForSkill` (make `/Game/CJW/Blueprints/Skill/S_Note` true _twice_2 _triple_2 _quad_2 _fifth))
      ;[1 1 1] 위젯 정보 초기화
      (`/Game/CJW/Blueprints/UI/Widget/WBP_Staff.UpdatePlayerNoteInfo` (`/Game/CJW/Blueprints/UI/Actor/BP_Staff.As WBP Staff` (`self.Staff`)) (`self.NoteForSkill`)))
    (:`NewEnumerator2`
      (set `self.NoteForSkill` (make `/Game/CJW/Blueprints/Skill/S_Note` _once_3 true _triple_3 _quad_3 _fifth_2))
      (`/Game/CJW/Blueprints/UI/Widget/WBP_Staff.UpdatePlayerNoteInfo` (`/Game/CJW/Blueprints/UI/Actor/BP_Staff.As WBP Staff` (`self.Staff`)) (`self.NoteForSkill`)))
    (:`NewEnumerator3`
      (set `self.NoteForSkill` (make `/Game/CJW/Blueprints/Skill/S_Note` _once_4 _twice_4 true _quad_4 _fifth_3))
      (`/Game/CJW/Blueprints/UI/Widget/WBP_Staff.UpdatePlayerNoteInfo` (`/Game/CJW/Blueprints/UI/Actor/BP_Staff.As WBP Staff` (`self.Staff`)) (`self.NoteForSkill`)))
    (:`NewEnumerator5`
      (set `self.NoteForSkill` (make `/Game/CJW/Blueprints/Skill/S_Note` _once_5 _twice_5 _triple_5 true _fifth_4))
      (`/Game/CJW/Blueprints/UI/Widget/WBP_Staff.UpdatePlayerNoteInfo` (`/Game/CJW/Blueprints/UI/Actor/BP_Staff.As WBP Staff` (`self.Staff`)) (`self.NoteForSkill`)))
    (:`NewEnumerator6`
      (set `self.NoteForSkill` (make `/Game/CJW/Blueprints/Skill/S_Note` _once _twice _triple _quad true))
      (`/Game/CJW/Blueprints/UI/Widget/WBP_Staff.UpdatePlayerNoteInfo` (`/Game/CJW/Blueprints/UI/Actor/BP_Staff.As WBP Staff` (`self.Staff`)) (`self.NoteForSkill`)))))

(fn `HPSet`
  (params (Amount :type "Float (double-precision)") (bAdd :type Boolean))
  ;[1 1 1] 체력 회복 or 차감 관련 노드
  (if bAdd
    (set `self.Hp` (+ (`self.Hp`) Amount))
    (else
      (set `self.Hp` (- (`self.Hp`) Amount)))))

(fn `ScoreSet`
  (params (Amount :type "Float (double-precision)") (bAdd :type Boolean))
  ;[1 1 1] 체력 회복 or 차감 관련 노드
  (if bAdd
    (set `self.Score` (+ (`self.Score`) Amount))
    (else
      (set `self.Score` (- (`self.Score`) Amount)))))

(fn `StartSetting`
  ;[1 1 1] 시작했을때 세팅 ,Staff와 Staff 위젯 정보 가져와서 져장
  (bind _returnvalue (`GameplayStatics.GetActorOfClass` "/Game/CJW/Blueprints/UI/Actor/BP_Staff.BP_Staff_C"))
  (set `self.Staff` _returnvalue))

(fn `UpdateSplineMesh`
  (bind _spline (`self.Spline`))
  (bind (_location _tangent) (`SplineComponent.GetLocationAndTangentAtSplinePoint` _spline 1 "Local"))
  (bind (_location_2 _tangent_2) (`SplineComponent.GetLocationAndTangentAtSplinePoint` _spline 0 "Local"))
  ;[1 1 1] 해당함수가 울리면 선형 보간을 실행시켜 부드럽게 레이저가 발사되도록한다
  (`SplineMeshComponent.SetStartAndEnd` (`self.SplineMesh`) _location_2 _tangent_2 _location _tangent true))

(fn `UserConstructionScript`)