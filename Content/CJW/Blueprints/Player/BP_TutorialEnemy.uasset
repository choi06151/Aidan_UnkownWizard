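; BP_TutorialEnemy is a training target that completes one step of the tutorial when the player's basic attack hits it.
; On BeginPlay it finds the BP_TrainingTextBox, and on overlap with BP_PlayerBasicAttack it checks the text widget's prompt index.
; At the matching hard-coded index it calls MissionClear and destroys itself.
; A GoToLocation event moves it to a fixed X/Y, with a timeline driving its height.
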(event `self.ReceiveBeginPlay`
  (bind _returnvalue (`GameplayStatics.GetActorOfClass` "/Game/CJW/Blueprints/UI/Actor/BP_TrainingTextBox.BP_TrainingTextBox_C"))
  (set `self.TrainingBox` _returnvalue))

(event `self.ReceiveActorBeginOverlap`
  (params (OtherActor :type "Actor Object Reference"))
  (bind _as_wbp_tutorial_text (`/Game/CJW/Blueprints/UI/Actor/BP_TrainingTextBox.As WBP Tutorial Text` (`self.TrainingBox`)))
  (cast `/Game/CJW/Blueprints/Bullet/BulletPool/BP_PlayerBasicAttack` OtherActor)
  (if (== (`/Game/CJW/Blueprints/UI/Widget/WBP_TutorialText.CurrentPromptIndex` _as_wbp_tutorial_text) 9)
    (`/Game/CJW/Blueprints/UI/Widget/WBP_TutorialText.MissionClear` _as_wbp_tutorial_text)
    (`self.K2_DestroyActor`)))

(event `Go To Location`
  (bind (_direction _newtrack_0) (`Timeline|Timeline` :!via `PlayFromStart`)
    (:`Update`
      (`self.K2_SetActorLocation` (`KismetMathLibrary.MakeVector` 1540.0 750.0 _newtrack_0)))))

(fn `UserConstructionScript`)