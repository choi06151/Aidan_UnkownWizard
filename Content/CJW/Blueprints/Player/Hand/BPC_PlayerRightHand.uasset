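; Right-hand component that records, deletes and recognises named hand gestures stored in a save game.
; A looping timer compares component-space bone positions against saved poses within a threshold and fires OnGestureRecognisedRight when the match changes.
; Tick separately updates per-finger down flags from fingertip-to-socket distance, feeding only test prints.
; IsFingerDown computes that distance only in its Debug branch, which Tick leaves off.
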(event `self.ReceiveBeginPlay`
  ;[1 1 1] 제스쳐 감지 영역
  (set `self.Gesture` (`/Game/CJW/Blueprints/Player/Hand/Gesture/BP_SaveGameGestureRight.Gesture` (`self.LoadGesture`)))
  ;;[1 1 1] 0.1초마다 재감지
  (`KismetSystemLibrary.K2_SetTimerDelegate` (delegate `DetectGesture`) (`self.RefreshRate`) true))

(event `DetectGesture`
  ;[1 1 1] 제스쳐 감지 영역
  ;;[1 1 1] 현재행동을 비교하여
  (bind (_result _gesture) (`self.GetCurrentGesture`))
  (if _result
    ;;[1 1 1] 있는 제스쳐라면 실행
    (if (not (`self.EqualGestures` _gesture (`self.CurrentGesture`)))
      (bind _output_get (set `self.CurrentGesture` _gesture))
      (`self.OnGestureRecognisedRight` (`.GestureName_2_B5624E584462AD6E7196E1B9901D7949` (break `/Game/CJW/Blueprints/Player/Hand/Gesture/S_Gesture` _output_get))))))

(event `self.ReceiveTick`
  (params (DeltaSeconds :type "Float (single-precision)"))
  (`|ExecutionSequence`
    (:`then_0`
      ;[1 1 1] 손가락의 펴짐 좁혀짐 유무 판별 , 각 손가락 별 실시
      ;;[1 1 1] 검지
      (bind _returnvalue (`self.IsFingerDown` (`self.IndexTipBone`) (`self.IndexFingerSocket`)))
      (if _returnvalue
        (if (not (`self.bIndexDown`))
          (set `self.bIndexDown` (not (`self.bIndexDown`)) :!label _label))
        (elif (`self.bIndexDown`)
          (goto _label))))
    (:`then_1`
      (bind _returnvalue_2 (`self.IsFingerDown` (`self.MiddleTipBone`) (`self.MiddleFingerSocket`)))
      (if _returnvalue_2
        (if (not (`self.bMiddleDown`))
          (set `self.bMiddleDown` (not (`self.bMiddleDown`)) :!label _label_2))
        (elif (`self.bMiddleDown`)
          (goto _label_2))))
    (:`then_2`
      ;;[1 1 1] 약지
      (bind _returnvalue_3 (`self.IsFingerDown` (`self.RingTipBone`) (`self.RingFingerSocket`)))
      (if _returnvalue_3
        (if (not (`self.bRingDown`))
          (set `self.bRingDown` (not (`self.bRingDown`)) :!label _label_3))
        (elif (`self.bRingDown`)
          (goto _label_3))))
    (:`then_3`
      ;;[1 1 1] 새끼
      (bind _returnvalue_4 (`self.IsFingerDown` (`self.PinkyTipBone`) (`self.PinkyFingerSocket`)))
      (if _returnvalue_4
        (if (not true)
          (set `self.bPinkyDown` (not (`self.bPinkyDown`)) :!label _label_4))
        (elif (`self.bPinkyDown`)
          (goto _label_4))))
    (:`then_4`
      ;;[1 1 1] 검지
      (bind _returnvalue_5 (`self.IsFingerDown` (`self.TunmbTipBone`) (`self.TunmbFingerSocket`)))
      (if _returnvalue_5
        (if (not (`self.bTunmbDown`))
          (set `self.bTunmbDown` (not (`self.bTunmbDown`)) :!label _label_5))
        (elif (`self.bTunmbDown`)
          (goto _label_5))))
    (:`then_5`
      (if (and (`self.bMiddleDown`) (`self.bRingDown`))
        (`KismetSystemLibrary.PrintString` "Hello")
        (else
          (set `self.TestRight` false)
          (`KismetSystemLibrary.PrintString` "no"))))))

(fn `DeleteGesture`
  (params (GestureName :type String))
  (locals (GestureSaveGame :type "/Game/CJW/Blueprints/Player/Hand/Gesture/BP_SaveGameGestureRight Object Reference") (Index :type Integer))
  ;[1 1 1] 제스쳐 파일 가져와서
  (bind _output_get (set `local.GestureSaveGame` (`self.LoadGesture`)))
  (for (_array_element _array_index) (`/Game/CJW/Blueprints/Player/Hand/Gesture/BP_SaveGameGestureRight.Gesture` _output_get)
    ;[1 1 1] 요구한 이름과 같은 제스쳐정보를 가져와서
    (if (== (`.GestureName_2_B5624E584462AD6E7196E1B9901D7949` (break `/Game/CJW/Blueprints/Player/Hand/Gesture/S_Gesture` _array_element)) GestureName)
      (set `local.Index` _array_index)))
  ;[1 1 1] 삭제하고 다시 저장
  (`KismetArrayLibrary.Array_Remove` (`/Game/CJW/Blueprints/Player/Hand/Gesture/BP_SaveGameGestureRight.Gesture` (`local.GestureSaveGame`)) (`local.Index`))
  (`GameplayStatics.SaveGameToSlot` (`local.GestureSaveGame`) (`self.GestureGameSlot`)))

(fn `DoesGestureExist?`
  (params (SaveGameGesture :type "/Game/CJW/Blueprints/Player/Hand/Gesture/BP_SaveGameGestureRight Object Reference") (GestureName :type String))
  (returns (Result :type Boolean))
  ;[1 1 1] 이미 존재하는 제스쳐를 저장하지 않기 위함 검사
  (for _array_element (`/Game/CJW/Blueprints/Player/Hand/Gesture/BP_SaveGameGestureRight.Gesture` SaveGameGesture)
    (if (== (`.GestureName_2_B5624E584462AD6E7196E1B9901D7949` (break `/Game/CJW/Blueprints/Player/Hand/Gesture/S_Gesture` _array_element)) GestureName)
      (return true)))
  (return false))

(fn `EqualGestures`
  (params (A :type "/Game/CJW/Blueprints/Player/Hand/Gesture/S_Gesture Structure") (B :type "/Game/CJW/Blueprints/Player/Hand/Gesture/S_Gesture Structure"))
  (returns (ReturnValue :type Boolean))
  (bind (_gesturename _bonelocation) (break `/Game/CJW/Blueprints/Player/Hand/Gesture/S_Gesture` A))
  (bind (_gesturename_2 _bonelocation_2) (break `/Game/CJW/Blueprints/Player/Hand/Gesture/S_Gesture` B))
  ;[1 1 1] 제스쳐 비교 하여 맞으면 참 아니면 거짓 반환
  (return (and (== _gesturename _gesturename_2) (`KismetArrayLibrary.Array_Identical` _bonelocation _bonelocation_2))))

(fn `GetCurrentGesture`
  (returns (Result :type Boolean) (Gesture :type "/Game/CJW/Blueprints/Player/Hand/Gesture/S_Gesture Structure"))
  (locals (bValidGesture :type Boolean :default true))
  ;[1 1 1] 현재 제스쳐 감지
  ;[1 1 1] 제스쳐에 저장된 슬롯을 하나씩 비교해 보면서
  (for _array_element (`self.Gesture`)
    (for (_array_element_2 _array_index) (`.BoneLocation_6_85C77533478A11029A4CF1907F014B4B` (break `/Game/CJW/Blueprints/Player/Hand/Gesture/S_Gesture` _array_element))
      ;[1 1 1] 저장된 값과 , 현재의 값을 비교하여
      (bind _returnvalue (`self.GetBoneLocationByName` (`self.GetBoneName` _array_index) "ComponentSpace"))
      (if (not (`self.Debug`))
        ;[1 1 1] 유효한 제스쳐가 아님을 (없는 제스쳐 )
        (if (> (`KismetMathLibrary.Abs` (`KismetMathLibrary.VSize` (- _returnvalue _array_element_2))) (`self.ThresholdForGesture`))
          (set `local.bValidGesture` false))))
    ;[1 1 1] 없는 재스쳐를 취한다면
    (if (`local.bValidGesture`)
      ;[1 1 1] 그때의 아닌 제스쳐를 반환하고
      (return (`local.bValidGesture`) _array_element)
      (else
        ;[1 1 1] 유효하다면 다시 키기
        (set `local.bValidGesture` true)))))

(fn `IsFingerDown`
  (params (BoneName :type Name) (SocketName :type Name) (Debug :type Boolean))
  (returns (ReturnValue :type Boolean))
  (bind _returnvalue (`self.GetSocketLocation` SocketName))
  (bind _returnvalue_2 (`self.GetBoneLocationByName` BoneName "WorldSpace"))
  (if Debug
    ;[1 1 1] 1.손톱위치 .2. 접었을때 손톱위치3.bool값,임계값
    (`KismetSystemLibrary.DrawDebugPoint` _returnvalue_2 20.0 (struct :`R` 1.0 :`A` 1.0) 0.1)
    (`KismetSystemLibrary.DrawDebugPoint` _returnvalue 20.0 (struct :`G` 1.0 :`A` 1.0) 0.1)
    (bind _returnvalue_3 (< (`KismetMathLibrary.Abs` (`KismetMathLibrary.VSize` (- _returnvalue_2 _returnvalue))) (`self.ThresholdForFingerDown`)))
    (`KismetSystemLibrary.PrintString` (`KismetStringLibrary.Concat_StrStr` (`KismetStringLibrary.Conv_BoolToString` _returnvalue_3)))
    (return _returnvalue_3)))

(fn `LoadGesture`
  (returns (Output :type "/Game/CJW/Blueprints/Player/Hand/Gesture/BP_SaveGameGestureRight Object Reference"))
  ;[1 1 1] 존재 유무 확인
  (bind _returnvalue (`GameplayStatics.DoesSaveGameExist` (`self.GestureGameSlot`)))
  (if _returnvalue
    ;[1 1 1] 존재한다면 , 거기에 저장
    (bind _returnvalue_2 (`GameplayStatics.LoadGameFromSlot` (`self.GestureGameSlot`)))
    (bind _asbp_save_game_gesture_right (cast `/Game/CJW/Blueprints/Player/Hand/Gesture/BP_SaveGameGestureRight` _returnvalue_2))
    (return _asbp_save_game_gesture_right)
    (else
      ;[1 1 1] 존재하지 않는다면 만들어서 저장
      (bind _returnvalue_3 (`GameplayStatics.CreateSaveGameObject` "/Game/CJW/Blueprints/Player/Hand/Gesture/BP_SaveGameGestureRight.BP_SaveGameGestureRight_C"))
      (return _returnvalue_3))))

(fn `RecordGesture`
  (params (GestureName :type String))
  (locals (GestureSaveGame :type "/Game/CJW/Blueprints/Player/Hand/Gesture/BP_SaveGameGestureRight Object Reference") (BoneLocations :type "Array of Vector Structure"))
  ;[1 1 1] 제스처를 저장하기위 저장공간 가져오기
  (bind _output_get (set `local.GestureSaveGame` (`self.LoadGesture`)))
  ;[1 1 1] 중복된 제스쳐를 받지 않기 위한 If
  (if (not (`self.DoesGestureExist?` _output_get GestureName))
    (for _index (range (`self.GetNumBones`))
      ;[1 1 1] 제스쳐 행동동안 모든 뼈 위치를 가져와서 BoneLocation에 추가
      (bind _returnvalue (`self.GetBoneLocationByName` (`self.GetBoneName` _index) "ComponentSpace"))
      (`KismetArrayLibrary.Array_Add` (`local.BoneLocations`) _returnvalue))
    ;[1 1 1] 녹음이 완료되면 제스쳐를 추가하고 , 해당 제스쳐를 슬롯에 저장
    (`KismetArrayLibrary.Array_Add` (`/Game/CJW/Blueprints/Player/Hand/Gesture/BP_SaveGameGestureRight.Gesture` (`local.GestureSaveGame`)) (make `/Game/CJW/Blueprints/Player/Hand/Gesture/S_Gesture` (`local.GestureName`) (`local.BoneLocations`)))
    (`GameplayStatics.SaveGameToSlot` (`local.GestureSaveGame`) (`self.GestureGameSlot`))))