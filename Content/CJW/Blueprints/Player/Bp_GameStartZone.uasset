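; Game start trigger zone that begins the spawning phase when the boss enters it.
; On BeginPlay it caches the player pawn as BP_Player and the game mode as VRGameMode.
; A BP_Boss overlap immediately changes the player's current status, then after a ten-second delay sets the game mode's StartSpawn flag.
; Overlaps from any other actor are ignored.
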(event `self.ReceiveBeginPlay`
  (bind _asbp_player (cast `/Game/CJW/Blueprints/Player/BP_Player` (`GameplayStatics.GetPlayerPawn` 0)))
  (set `self.As BP Player` _asbp_player)
  (bind _asvrgame_mode (cast `/Game/VRTemplate/Blueprints/VRGameMode` (`GameplayStatics.GetGameMode`)))
  (set `self.As VRGame Mode` _asvrgame_mode))

(event `self.ReceiveActorBeginOverlap`
  (params (OtherActor :type "Actor Object Reference"))
  (cast `/Game/JWK/00_BP/BP_Boss` OtherActor)
  (set `/Game/CJW/Blueprints/Player/BP_Player.CurrentPlayerStatus` "NewEnumerator1" (`self.As BP Player`))
  (`KismetSystemLibrary.Delay` 10.0)
  (set `/Game/VRTemplate/Blueprints/VRGameMode.bStartSpawn` true (`self.As VRGame Mode`)))

(fn `UserConstructionScript`)