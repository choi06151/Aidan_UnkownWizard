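; Homing note-bullet projectile that picks one of five types at BeginPlay, setting its mesh and dynamic material.
; ActiveBullet launches it at the player with a timeout; staff in the required state dissolves it and receives its type, while player hits deal damage.
; Those hits, break zones and timeout deactivate it without destroying and notify listeners.
; Extra events drive a material-based black-hole effect, delayed hiding, tutorial placement and retargeting.
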(event `self.ReceiveBeginPlay`
  (bind _output (`|GetArrayItem` (`self.Materials`) 4))
  (bind _output_2 (`|GetArrayItem` (`self.Materials`)))
  (bind _output_3 (`|GetArrayItem` (`self.Materials`) 2))
  (bind _output_4 (`|GetArrayItem` (`self.Materials`) 3))
  ;[1 1 1] 태어났을때 5가지의 타입중 하나를 선택하여 랜덤타입 결정
  (bind _output_get (set `self.CurrentType` (`KismetArrayLibrary.Array_Random` (`self.EntireType`)) :!label _label))
  (switch `/Game/CJW/Blueprints/Skill/E_NoteType` _output_get
    (:`NewEnumerator0`
      (goto _label))
    (:`NewEnumerator1`
      (`StaticMeshComponent.SetStaticMesh` (`self.BulletMesh`) (`|GetArrayItem` (`self.Meshes`)))
      (`PrimitiveComponent.SetMaterial` (`self.BulletMesh`) 0 _output_2)
      (bind _returnvalue (`PrimitiveComponent.CreateDynamicMaterialInstance` (`self.BulletMesh`) 0 _output_2 "None"))
      (set `self.DynamicMaterial` _returnvalue))
    (:`NewEnumerator2`
      (`StaticMeshComponent.SetStaticMesh` (`self.BulletMesh`) (`|GetArrayItem` (`self.Meshes`) 1))
      (`PrimitiveComponent.SetMaterial` (`self.BulletMesh`) 0 (`|GetArrayItem` (`self.Materials`) 1))
      (bind _returnvalue_2 (`PrimitiveComponent.CreateDynamicMaterialInstance` (`self.BulletMesh`) 0 null "None"))
      (set `self.DynamicMaterial` _returnvalue_2))
    (:`NewEnumerator3`
      (`StaticMeshComponent.SetStaticMesh` (`self.BulletMesh`) (`|GetArrayItem` (`self.Meshes`) 2))
      (`PrimitiveComponent.SetMaterial` (`self.BulletMesh`) 0 _output_3)
      (bind _returnvalue_3 (`PrimitiveComponent.CreateDynamicMaterialInstance` (`self.BulletMesh`) 0 _output_3 "None"))
      (set `self.DynamicMaterial` _returnvalue_3))
    (:`NewEnumerator5`
      (`StaticMeshComponent.SetStaticMesh` (`self.BulletMesh`) (`|GetArrayItem` (`self.Meshes`) 3))
      (`PrimitiveComponent.SetMaterial` (`self.BulletMesh`) 0 _output_4)
      (bind _returnvalue_4 (`PrimitiveComponent.CreateDynamicMaterialInstance` (`self.BulletMesh`) 0 _output_4 "None"))
      (set `self.DynamicMaterial` _returnvalue_4))
    (:`NewEnumerator6`
      (`StaticMeshComponent.SetStaticMesh` (`self.BulletMesh`) (`|GetArrayItem` (`self.Meshes`) 4))
      (`PrimitiveComponent.SetMaterial` (`self.BulletMesh`) 0 _output)
      (bind _returnvalue_5 (`PrimitiveComponent.CreateDynamicMaterialInstance` (`self.BulletMesh`) 0 _output "None"))
      (set `self.DynamicMaterial` _returnvalue_5))))

(event `StartDissolve`
  ;[1 1 1] 디솔브
  (bind (_direction _newtrack_0) (`Timeline|Timeline` :!via `PlayFromStart`)
    (:`Update`
      (`MeshComponent.SetScalarParameterValueOnMaterials` (`self.BulletMesh`) "Dissolve" _newtrack_0))))

(event `OnStop`
  ;[1 1 1] 궁극기 맞았을때 사라지게
  (`KismetSystemLibrary.Delay` 0.2)
  (`self.SetActorHiddenInGame` true))

(event `StartBlackHoling`
  (params (Location :type "Vector Structure"))
  (bind _dynamicmaterial (`self.DynamicMaterial`))
  ;[1 1 1] 크레센도 맞았을때 효과
  (bind (_direction _newtrack_0) (`Timeline|Timeline_0` :!via `PlayFromStart`)
    (:`Update`
      (`MaterialInstanceDynamic.SetVectorParameterValue` _dynamicmaterial "blackholepos" (`KismetMathLibrary.Conv_VectorToLinearColor` Location))
      (`MaterialInstanceDynamic.SetScalarParameterValue` _dynamicmaterial "ScaleValue" _newtrack_0)
      (`MaterialInstanceDynamic.SetScalarParameterValue` _dynamicmaterial "Radius" 600.0)
      (`MaterialInstanceDynamic.SetScalarParameterValue` _dynamicmaterial "TransitionLength" 0.5))
    (:`Finished`
      (`self.SetActorHiddenInGame` true))))

(event `self.BulletMesh.OnComponentBeginOverlap`
  (params (OverlappedComponent :type "PrimitiveComponent Object Reference") (OtherActor :type "Actor Object Reference") (OtherComp :type "PrimitiveComponent Object Reference") (OtherBodyIndex :type Integer) (bFromSweep :type Boolean) (SweepResult :type "HitResult Structure (by ref)")))

(event `self.ReceiveActorBeginOverlap`
  (params (OtherActor :type "Actor Object Reference"))
  ;[1 1 1] 2차 조건 Staff 일때
  (bind _asbp_staff (cast `/Game/CJW/Blueprints/UI/Actor/BP_Staff` OtherActor)
    (:`then`
      (if (`|EnumEquality` (`/Game/CJW/Blueprints/UI/Actor/BP_Staff.CurrentState` _asbp_staff) "NewEnumerator1")
        (`self.StartDissolve`)
        (`/Game/CJW/Blueprints/Player/BP_Player.GetNoteInfo` (`/Game/CJW/Blueprints/UI/Actor/BP_Staff.BP Player Info` _asbp_staff) (`self.CurrentType`))
        (`self.DeactiveBullet`)
        (`self.OnNoteBulletDestroyed` self)))
    (:`CastFailed`
      ;[1 1 1] 1차 조건 , 플레이어일때
      (bind _asbp_player (cast `/Game/CJW/Blueprints/Player/BP_Player` OtherActor)
        (:`then`
          (`GameplayStatics.ApplyDamage` _asbp_player (`self.Damage`) null self)
          (`self.DeactiveBullet`)
          (`self.OnNoteBulletDestroyed` self))
        (:`CastFailed`
          ;[1 1 1] 3차조건 , 마무리
          (cast `/Game/CJW/Blueprints/Bullet/BP_BreakZone` OtherActor)
          (`self.DeactiveBullet`)
          (`self.OnNoteBulletDestroyed` self))))))

(event `ActiveBullet`
  (params (Velocity :type "Vector Structure") (`Spawn Location` :type "Vector Structure"))
  (bind _projectilemovement (`self.ProjectileMovement`))
  ;[1 1 1] 총알 활성화
  (`self.K2_SetActorLocation` `Spawn Location` false true)
  (`self.SetActorHiddenInGame` false)
  (set `MovementComponent.Velocity` Velocity (`self.ProjectileMovement`))
  (`PrimitiveComponent.SetCollisionEnabled` (`self.BulletMesh`) "QueryOnly")
  ;[1 1 1] 호밍 프로젝타일 사용 , 태어날때 받은 스피드를 기준으로 플레이어를 따라다닌다
  (set `ProjectileMovementComponent.bIsHomingProjectile` true _projectilemovement)
  (set `ProjectileMovementComponent.HomingTargetComponent` (`Actor.RootComponent` (`GameplayStatics.GetPlayerPawn` 0)) _projectilemovement)
  (set `ProjectileMovementComponent.HomingAccelerationMagnitude` (`self.Speed`) _projectilemovement)
  (`KismetSystemLibrary.Delay` 5.0)
  (`self.DeactiveBullet`)
  (`self.OnNoteBulletDestroyed` self))

(event `DeactiveBullet`
  ;[1 1 1] 총알 비활성화
  (set `ProjectileMovementComponent.HomingAccelerationMagnitude` 0.0 (`self.ProjectileMovement`))
  (set `MovementComponent.Velocity` (0.0 0.0 0.0) (`self.ProjectileMovement`))
  (`PrimitiveComponent.SetCollisionEnabled` (`self.BulletMesh`) "NoCollision"))

(event `Set Loc to Display`
  ;[1 1 1] 지정된 위치로 이동
  (bind _outactors (`GameplayStatics.GetAllActorsOfClass` "/Script/Engine.TargetPoint"))
  (for _array_element _outactors
    (if (`self.ActorHasTag` _array_element "Tutorial2")
      (`self.K2_SetActorLocation` (`self.K2_GetActorLocation` _array_element) false true)
      (`KismetSystemLibrary.PrintString` "Spawn!!"))))

(event `GotoPlayer`
  (bind _projectilemovement (`self.ProjectileMovement`))
  ;[1 1 1] 플레이어 한테 돌격
  (bind _returnvalue (`GameplayStatics.GetActorOfClass` "/Game/CJW/Blueprints/Player/BP_Player.BP_Player_C"))
  (set `ProjectileMovementComponent.bIsHomingProjectile` true _projectilemovement)
  (set `ProjectileMovementComponent.HomingTargetComponent` (`Actor.RootComponent` _returnvalue) _projectilemovement)
  (set `ProjectileMovementComponent.HomingAccelerationMagnitude` 2000.0 _projectilemovement))

(event `GotoPlayerDirection`
  (bind _projectilemovement (`self.ProjectileMovement`))
  (`KismetSystemLibrary.Delay` 3.0)
  (bind _returnvalue (`GameplayStatics.GetActorOfClass` "/Game/CJW/Blueprints/Bullet/BP_Target.BP_Target_C"))
  (set `ProjectileMovementComponent.bIsHomingProjectile` true _projectilemovement)
  (set `ProjectileMovementComponent.HomingTargetComponent` (`Actor.RootComponent` _returnvalue) _projectilemovement)
  (set `ProjectileMovementComponent.HomingAccelerationMagnitude` 2000.0 _projectilemovement))

(fn `UserConstructionScript`)