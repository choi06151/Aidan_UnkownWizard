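; BP_BreakZone is an overlap trigger that hides actors entering it and can complete a training tutorial mission.
; On BeginPlay it caches the level's BP_TrainingTextBox to reach the tutorial text widget.
; Overlaps from anything except BP_SpawnUI call MissionClear if the tutorial is at prompt 16, then hide the other actor.
; The zone then disables its own collision, so it stops responding after the first qualifying overlap.
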(event `self.ReceiveBeginPlay`
  (bind _returnvalue (`GameplayStatics.GetActorOfClass` "/Game/CJW/Blueprints/UI/Actor/BP_TrainingTextBox.BP_TrainingTextBox_C"))
  (set `self.Trainingbox` _returnvalue))

(event `self.ReceiveActorBeginOverlap`
  (params (OtherActor :type "Actor Object Reference"))
  (bind _as_wbp_tutorial_text (`/Game/CJW/Blueprints/UI/Actor/BP_TrainingTextBox.As WBP Tutorial Text` (`self.Trainingbox`)))
  (cast `/Game/SEB/Blueprints/BP_SpawnUI` OtherActor
    (:`CastFailed`
      (if (== (`/Game/CJW/Blueprints/UI/Widget/WBP_TutorialText.CurrentPromptIndex` _as_wbp_tutorial_text) 16)
        (`/Game/CJW/Blueprints/UI/Widget/WBP_TutorialText.MissionClear` _as_wbp_tutorial_text))
      (`self.SetActorHiddenInGame` OtherActor true)
      (`self.SetActorEnableCollision` false))))

(fn `UserConstructionScript`)