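; Component that pre-spawns and recycles two kinds of player projectile, basic attacks and paralyze (mute skill) shots, to serve as object pools.
; On BeginPlay it spawns each type with its speed and damage, then stores it hidden, collision-disabled and attached to the owner.
; Each bullet's destroyed event is bound to a return handler that hides it, moves it back to the owner and reattaches it.
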(event `self.ReceiveBeginPlay`
  ;[1 1 1] 최초 생성 , 총알 저장
  (`|ExecutionSequence`
    (:`then_0`
      (for _ (range (+ (`self.PlayerBasicBulletAmountOfBullets`) 1))
        (bind _returnvalue (`|SpawnActorFromClass` "/Game/CJW/Blueprints/Bullet/BulletPool/BP_PlayerBasicAttack.BP_PlayerBasicAttack_C" (`KismetMathLibrary.MakeTransform` (`Actor.K2_GetActorLocation` (`self.GetOwner`))) "Undefined" "MultiplyWithRoot" null (`self.BasicAttackSpeed`) (`self.BasicAttackDamage`) null))
        (`PrimitiveComponent.SetCollisionEnabled` (`/Game/CJW/Blueprints/Bullet/BulletPool/BP_PlayerBasicAttack.BulletMesh` _returnvalue) "NoCollision")
        (`Actor.K2_AttachToActor` _returnvalue (`self.GetOwner`) "None" "KeepWorld" "KeepWorld" "KeepWorld" true)
        (`Actor.SetActorHiddenInGame` _returnvalue true)
        ;[1 1 1] Destroy 대신 pool로 다시 돌아오는 함수
        (add `/Game/CJW/Blueprints/Bullet/BulletPool/BP_PlayerBasicAttack.OnPlayerBasicBulletDestroyed` _returnvalue (delegate `ReturnToPool`))
        (`KismetArrayLibrary.Array_Add` (`self.PlayerBasicBulletPool`) _returnvalue)))
    (:`then_1`
      (for _ (range (+ (`self.PlayerPalarizeAmountOfBullet`) 1))
        (bind _returnvalue_2 (`|SpawnActorFromClass` "/Game/CJW/Blueprints/Bullet/BulletPool/BP_PlayerMuteSkill.BP_PlayerMuteSkill_C" (`KismetMathLibrary.MakeTransform` (`Actor.K2_GetActorLocation` (`self.GetOwner`))) "Undefined" "MultiplyWithRoot" null (`self.PalarizeAttackSpeed`) (`self.PalarizeAttackDamage`) null))
        (`PrimitiveComponent.SetCollisionEnabled` (`/Game/CJW/Blueprints/Bullet/BulletPool/BP_PlayerMuteSkill.BulletMesh` _returnvalue_2) "NoCollision")
        (`Actor.K2_AttachToActor` _returnvalue_2 (`self.GetOwner`) "None" "KeepWorld" "KeepWorld" "KeepWorld" true)
        (`Actor.SetActorHiddenInGame` _returnvalue_2 true)
        (add `/Game/CJW/Blueprints/Bullet/BulletPool/BP_PlayerMuteSkill.OnPlayerParlarizeDestroyed` _returnvalue_2 (delegate `PaLReturnToPool`))
        (`KismetArrayLibrary.Array_Add` (`self.PlayerPalarizeBulletPool`) _returnvalue_2)))))

(event `ReturnToPool`
  (params (Bullet :type "/Game/CJW/Blueprints/Bullet/BulletPool/BP_PlayerBasicAttack Object Reference"))
  (bind _returnvalue (`self.GetOwner`))
  ;[1 1 1] Destroy 대신 pool로 다시 돌아오는 함수
  (`Actor.SetActorHiddenInGame` Bullet true)
  (`Actor.SetActorScale3D` Bullet (0.5 0.5 0.5))
  (`Actor.K2_SetActorLocation` Bullet (`Actor.K2_GetActorLocation` _returnvalue) false true)
  (`Actor.K2_AttachToActor` Bullet _returnvalue "None" "KeepWorld" "KeepWorld" "KeepWorld" true))

(event `PaLReturnToPool`
  (params (Bullet :type "/Game/CJW/Blueprints/Bullet/BulletPool/BP_PlayerMuteSkill Object Reference"))
  (bind _returnvalue (`self.GetOwner`))
  (`Actor.K2_SetActorLocation` Bullet (`Actor.K2_GetActorLocation` _returnvalue) false false)
  (`Actor.K2_AttachToActor` Bullet _returnvalue "None" "KeepWorld" "KeepWorld" "KeepWorld" true)
  (`Actor.SetActorHiddenInGame` Bullet true))