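; BP_PlayerMuteSkill is a reusable projectile for the player's Mute skill that homes in on BP_Boss.
; On BeginPlay it caches TargetPoints tagged "Mute" and the boss; ActiveBullet moves it to a random cached point, shows it, attaches particles and starts homing.
; On boss overlap it applies delayed damage, disables collision, calls OnPlayerParlarizeDestroyed, shakes the camera and swaps the trail for a spawned effect.
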(event `self.ReceiveBeginPlay`
  (bind _projectilemovement (`self.ProjectileMovement`))
  (set `ProjectileMovementComponent.InitialSpeed` (`self.AttackSpeed`) _projectilemovement)
  (set `ProjectileMovementComponent.MaxSpeed` (`self.AttackSpeed`) _projectilemovement)
  (bind _outactors (`GameplayStatics.GetAllActorsOfClass` "/Script/Engine.TargetPoint"))
  (for _array_element _outactors
    (if (`self.ActorHasTag` _array_element "Mute")
      (`KismetArrayLibrary.Array_Add` (`self.SpawnPoint`) _array_element)
      (bind _returnvalue (`GameplayStatics.GetActorOfClass` "/Game/JWK/00_BP/BP_Boss.BP_Boss_C"))
      (set `self.Target` _returnvalue))))

(event `self.ReceiveTick`
  (params (DeltaSeconds :type "Float (single-precision)")))

(event `ActiveBullet`
  (params (AttackDamage :type "Float (double-precision)") (`Attack Scale` :type "Vector Structure"))
  (bind _projectilemovement (`self.ProjectileMovement`))
  ;[1 1 1] 총알 활성화
  (set `self.AttackDamage` AttackDamage)
  (`self.SetActorScale3D` `Attack Scale`)
  (`self.K2_SetActorLocation` (`self.K2_GetActorLocation` (`|GetArrayItem` (`self.SpawnPoint`) (`KismetMathLibrary.RandomInteger` (`KismetArrayLibrary.Array_Length` (`self.SpawnPoint`))))) false true)
  (`self.SetActorHiddenInGame` false)
  (set `MovementComponent.Velocity` (0.0 0.0 0.0) (`self.ProjectileMovement`))
  (`PrimitiveComponent.SetCollisionEnabled` (`self.BulletMesh`) "QueryOnly")
  (set `ProjectileMovementComponent.bIsHomingProjectile` true (`self.ProjectileMovement`))
  (set `ProjectileMovementComponent.HomingTargetComponent` (`Actor.RootComponent` (`self.Target`)) _projectilemovement)
  (set `ProjectileMovementComponent.HomingAccelerationMagnitude` 30000.0 _projectilemovement)
  (bind _returnvalue (`GameplayStatics.SpawnEmitterAttached` "/Game/CJW/VFX/Par_Meteora_01.Par_Meteora_01" (`self.BulletMesh`))))

(event `DeactiveBullet`
  ;[1 1 1] 총알 비활성화
  (set `MovementComponent.Velocity` (0.0 0.0 0.0) (`self.ProjectileMovement`))
  (`PrimitiveComponent.SetCollisionEnabled` (`self.BulletMesh`) "NoCollision"))

(event `self.BulletMesh.OnComponentBeginOverlap`
  (params (OverlappedComponent :type "PrimitiveComponent Object Reference") (OtherActor :type "Actor Object Reference") (OtherComp :type "PrimitiveComponent Object Reference") (OtherBodyIndex :type Integer) (bFromSweep :type Boolean) (SweepResult :type "HitResult Structure (by ref)"))
  (bind _asbp_boss (cast `/Game/JWK/00_BP/BP_Boss` OtherActor))
  (`KismetSystemLibrary.Delay` 0.7)
  (`GameplayStatics.ApplyDamage` _asbp_boss (`self.AttackDamage`) null self)
  (`self.DeactiveBullet`)
  (`self.OnPlayerParlarizeDestroyed` self)
  (`PlayerCameraManager.StartCameraShake` :`self` (`GameplayStatics.GetPlayerCameraManager` 0) :`ShakeClass` "/Game/CJW/CameraShake/CSB_Cresendo.CSB_Cresendo_C" :`Scale` 5.0)
  (`ActorComponent.K2_DestroyComponent` (stale `ActiveBullet` _returnvalue))
  (`GameplayStatics.SpawnEmitterAtLocation` null))

(fn `UserConstructionScript`)