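; BP_GameModeBulletPool pre-spawns a pool of note bullets (BP_NodeForTest actors) at BeginPlay for reuse.
; Each is spawned with the configured note speed, has mesh collision disabled, is hidden, and is stored in NoteBulletPool.
; Each bullet's destroyed event is bound to NoteReturnToPool, which teleports it to the origin and hides it again.
; The event graph contains no logic for taking bullets out of the pool.
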(event `self.ReceiveBeginPlay`
  (for _ (range (+ (`self.NoteBulletAmounOfBullet`) 1))
    (bind _returnvalue (`|SpawnActorFromClass` "/Game/CJW/Blueprints/Skill/BP_NodeForTest.BP_NodeForTest_C" (`KismetMathLibrary.MakeTransform` (0.0 0.0 0.0)) "Undefined" "MultiplyWithRoot" null (`self.NoteSpeed`) null))
    (`PrimitiveComponent.SetCollisionEnabled` (`/Game/CJW/Blueprints/Skill/BP_NodeForTest.BulletMesh` _returnvalue) "NoCollision")
    (`Actor.SetActorHiddenInGame` _returnvalue true)
    (add `/Game/CJW/Blueprints/Skill/BP_NodeForTest.OnNoteBulletDestroyed` _returnvalue (delegate `NoteReturnToPool`))
    (`KismetArrayLibrary.Array_Add` (`self.NoteBulletPool`) _returnvalue)))

(event `NoteReturnToPool`
  (params (TargetBullet :type "/Game/CJW/Blueprints/Skill/BP_NodeForTest Object Reference"))
  (`Actor.K2_SetActorLocation` TargetBullet (0.0 0.0 0.0) false true)
  (`Actor.SetActorHiddenInGame` TargetBullet true))