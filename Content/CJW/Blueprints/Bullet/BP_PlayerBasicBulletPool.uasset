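; Bullet pool for the player's basic attack, pre-spawning BP_PlayerBasicAttack actors to reuse instead of destroying them.
; On BeginPlay it spawns the bullets at its owner with attack speed and damage, disables mesh collision, attaches them to the owner and stores them in BulletPool.
; Each bullet's destroyed dispatcher calls ReturnToPool, which moves it back to the owner and reattaches it.
; Firing logic is not in this graph.
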(event `self.ReceiveBeginPlay`
  ;[1 1 1] 최초 생성 , 총알 저장
  (for _ (range (+ (`self.AmountOfBullets`) 1))
    (bind _returnvalue (`|SpawnActorFromClass` "/Game/CJW/Blueprints/Bullet/BP_PlayerBasicAttack.BP_PlayerBasicAttack_C" (`KismetMathLibrary.MakeTransform` (`Actor.K2_GetActorLocation` (`self.GetOwner`))) "Undefined" "MultiplyWithRoot" null (`self.AttackSpeed`) (`self.AttackDamage`) null))
    (`PrimitiveComponent.SetCollisionEnabled` (`/Game/CJW/Blueprints/Bullet/BP_PlayerBasicAttack.BulletMesh` _returnvalue) "NoCollision")
    (`Actor.K2_AttachToActor` _returnvalue (`self.GetOwner`) "None" "KeepWorld" "KeepWorld" "KeepWorld" true)
    ;[1 1 1] Destroy 대신 pool로 다시 돌아오는 함수
    (add `/Game/CJW/Blueprints/Bullet/BP_PlayerBasicAttack.OnPlayerBasicBulletDestroyed` _returnvalue (delegate `ReturnToPool`))
    (`KismetArrayLibrary.Array_Add` (`self.BulletPool`) _returnvalue)))

(event `ReturnToPool`
  (params (Bullet :type "/Game/CJW/Blueprints/Bullet/BP_PlayerBasicAttack Object Reference"))
  (bind _returnvalue (`self.GetOwner`))
  ;[1 1 1] Destroy 대신 pool로 다시 돌아오는 함수
  (`Actor.K2_SetActorLocation` Bullet (`Actor.K2_GetActorLocation` _returnvalue) false false)
  (`Actor.K2_AttachToActor` Bullet _returnvalue "None" "KeepWorld" "KeepWorld" "KeepWorld" true))