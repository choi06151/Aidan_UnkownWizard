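; Player basic-attack bullet that can be switched on and off rather than destroyed.
; On BeginPlay, AttackSpeed sets the projectile movement's initial and max speed.
; ActiveBullet applies a given velocity and enables query-only mesh collision, while DeactiveBullet zeroes velocity and disables collision.
; A mesh overlap deactivates the bullet and broadcasts OnPlayerBasicBulletDestroyed with itself, without destroying the actor.
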(event `self.ReceiveBeginPlay`
  (bind _projectilemovement (`self.ProjectileMovement`))
  ;[1 1 1] 스폰될때 주어진 속도값에 따라 총알 속도 변화
  (set `ProjectileMovementComponent.InitialSpeed` (`self.AttackSpeed`) _projectilemovement)
  (set `ProjectileMovementComponent.MaxSpeed` (`self.AttackSpeed`) _projectilemovement))

(event `self.BulletMesh.OnComponentBeginOverlap`
  (params (OverlappedComponent :type "PrimitiveComponent Object Reference") (OtherActor :type "Actor Object Reference") (OtherComp :type "PrimitiveComponent Object Reference") (OtherBodyIndex :type Integer) (bFromSweep :type Boolean) (SweepResult :type "HitResult Structure (by ref)"))
  (`self.DeactiveBullet`)
  (`self.OnPlayerBasicBulletDestroyed` self))

(event `ActiveBullet`
  (params (Velocity :type "Vector Structure"))
  ;[1 1 1] 총알 활성화
  (set `MovementComponent.Velocity` Velocity (`self.ProjectileMovement`))
  (`PrimitiveComponent.SetCollisionEnabled` (`self.BulletMesh`) "QueryOnly"))

(event `DeactiveBullet`
  ;[1 1 1] 총알 비활성화
  (set `MovementComponent.Velocity` (0.0 0.0 0.0) (`self.ProjectileMovement`))
  (`PrimitiveComponent.SetCollisionEnabled` (`self.BulletMesh`) "NoCollision"))

(fn `UserConstructionScript`)