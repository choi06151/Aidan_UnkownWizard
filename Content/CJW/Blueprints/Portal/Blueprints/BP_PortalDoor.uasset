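; BP_PortalDoor is a portal door that toggles the player's post-process view whenever the first-person camera passes through it.
; On BeginPlay it moves in front of the BP_Player camera; Tick runs crossing and clipping checks while the player overlaps Detection.
; Crossing combines a dot-product side flip with a line-plane intersection, then swaps Entry's material and the camera's post-process material.
; PreventPlaneClipping nudges Entry away from a nearby camera.
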(event `self.ReceiveBeginPlay`
  (bind _asbp_player (cast `/Game/CJW/Blueprints/Player/BP_Player` (`GameplayStatics.GetPlayerPawn` 0)))
  (bind _output_get (set `self.As BP Player` _asbp_player))
  (bind _camera (`/Game/CJW/Blueprints/Player/BP_Player.Camera` _output_get))
  (`self.K2_SetActorRelativeLocation` (+ (`SceneComponent.K2_GetComponentLocation` _camera) (* (`SceneComponent.GetForwardVector` _camera) 100.0)) false true)
  (`self.K2_AttachToComponent` null "None" "KeepWorld" "KeepWorld" "KeepWorld"))

(event `self.ReceiveTick`
  (params (DeltaSeconds :type "Float (single-precision)"))
  (if (`PrimitiveComponent.IsOverlappingActor` (`self.Detection`) (`GameplayStatics.GetPlayerCharacter` 0))
    (`self.PreventPlaneClipping`)
    (bind _iscrossing1 (`self.HasCrossedDoor`))
    (if _iscrossing1
      (if (`self.bInverted`)
        (set `self.bInverted` false)
        (`PrimitiveComponent.SetMaterial` (`self.Entry`) 0 (`self.DoorMaterial`))
        (set `CameraComponent.PostProcessSettings` (make `PostProcessSettings` :`WeightedBlendables` (make `WeightedBlendables` (`|MakeArray` (make `WeightedBlendable` 1.0 "/Game/CJW/Blueprints/Portal/Materials/M_ThroghPortal/M_DefalutShader_PPM.M_DefalutShader_PPM")))) (`/Game/FirstPerson/Blueprints/BP_FirstPersonCharacter.FirstPersonCamera` (cast `/Game/FirstPerson/Blueprints/BP_FirstPersonCharacter` (`GameplayStatics.GetPlayerCharacter` 0) :!pure true)))
        (else
          (set `self.bInverted` true)
          (`PrimitiveComponent.SetMaterial` (`self.Entry`) 0 "/Game/CJW/Blueprints/Portal/Materials/M_ThroghPortal/M_DefalutShader.M_DefalutShader")
          (set `CameraComponent.PostProcessSettings` (make `PostProcessSettings` :`WeightedBlendables` (make `WeightedBlendables` (`|MakeArray` (make `WeightedBlendable` 1.0 (`self.PostProcessMaterial`))))) (`/Game/FirstPerson/Blueprints/BP_FirstPersonCharacter.FirstPersonCamera` (cast `/Game/FirstPerson/Blueprints/BP_FirstPersonCharacter` (`GameplayStatics.GetPlayerCharacter` 0) :!pure true))))))
    (else
      (set `self.bOvelapping` false))))

(fn `HasCrossedDoor`
  (returns (IsCrossing1 :type Boolean))
  (locals (IsInFront :type Boolean) (DoorPlane :type "Plane Structure") (IsCrossing :type Boolean :default false))
  (set `local.IsInFront` (>= (`KismetMathLibrary.Dot_VectorVector` (`SceneComponent.GetForwardVector` (`self.ForwardDirection`)) (- (`SceneComponent.K2_GetComponentLocation` (`/Game/FirstPerson/Blueprints/BP_FirstPersonCharacter.FirstPersonCamera` (cast `/Game/FirstPerson/Blueprints/BP_FirstPersonCharacter` (`GameplayStatics.GetPlayerCharacter` 0) :!pure true))) (`self.K2_GetActorLocation`))) 0.0))
  (bind _output_get (set `local.DoorPlane` (`KismetMathLibrary.MakePlaneFromPointAndNormal` (`self.K2_GetActorLocation`) (`SceneComponent.GetForwardVector` (`self.ForwardDirection`)))))
  ;[1 1 1] 플레이어가 지나가면
  (set `self.bIntersecting` (`.ReturnValue` (`KismetMathLibrary.LinePlaneIntersection` (`SceneComponent.K2_GetComponentLocation` (`/Game/FirstPerson/Blueprints/BP_FirstPersonCharacter.FirstPersonCamera` (cast `/Game/FirstPerson/Blueprints/BP_FirstPersonCharacter` (`GameplayStatics.GetPlayerCharacter` 0) :!pure true))) (`self.Last Position`) _output_get)))
  (set `local.IsCrossing` (or (and (`self.bIntersecting`) (not (`local.IsInFront`)) (`self.LastInFront`) (`self.bOvelapping`)) (and (`self.bIntersecting`) (`local.IsInFront`) (not (`self.LastInFront`)) (`self.bOvelapping`))))
  (set `self.LastInFront` (`local.IsInFront`))
  (set `self.Last Position` (`SceneComponent.K2_GetComponentLocation` (`/Game/FirstPerson/Blueprints/BP_FirstPersonCharacter.FirstPersonCamera` (cast `/Game/FirstPerson/Blueprints/BP_FirstPersonCharacter` (`GameplayStatics.GetPlayerCharacter` 0) :!pure true))))
  (set `self.bOvelapping` true)
  (return (`local.IsCrossing`)))

(fn `PreventPlaneClipping`
  (bind _returnvalue (`KismetMathLibrary.Dot_VectorVector` (`SceneComponent.GetForwardVector` (`self.ForwardDirection`)) (- (`SceneComponent.K2_GetComponentLocation` (`/Game/FirstPerson/Blueprints/BP_FirstPersonCharacter.FirstPersonCamera` (cast `/Game/FirstPerson/Blueprints/BP_FirstPersonCharacter` (`GameplayStatics.GetPlayerCharacter` 0) :!pure true))) (`self.K2_GetActorLocation`))))
  (if (and (>= _returnvalue -3.0) (<= _returnvalue 0.0))
    ;[1 1 1] Pushmesh back if Player is so close
    (`SceneComponent.K2_SetRelativeLocation` (`self.Entry`) (2.0 0.0 100.0) false false)
    (elif (and (>= _returnvalue 0.0) (<= _returnvalue 3.0))
      ;[1 1 1] Pushmesh back if Player is so close
      (`SceneComponent.K2_SetRelativeLocation` (`self.Entry`) (-2.0 0.0 100.0) false false)
      (else
        (`SceneComponent.K2_SetRelativeLocation` (`self.Entry`) (-0.0 0.0 100.0) false false)))))

(fn `UserConstructionScript`
  (`PrimitiveComponent.SetMaterial` (`self.Entry`) 0 (`self.DoorMaterial`)))