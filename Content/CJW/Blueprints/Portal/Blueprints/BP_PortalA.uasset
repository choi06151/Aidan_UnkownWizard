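; BP_PortalA is a one-way portal actor that teleports whatever overlaps its Box to BP_PortalB.
; BeginPlay caches the BP_PortalB instance found with GetActorOfClass.
; On overlap, the other actor moves to PortalB's SceneCaptureComponent2D location, takes its rotation from the sweep's HitActor, and a debug "Hello" prints.
; An Arrow-to-impact offset calculation is left unconnected, and NewFunction simply wraps a vector distance.
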(event `self.ReceiveBeginPlay`
  ;[1 1 1] portal B의 정보 가져와서 넣기
  (bind _returnvalue (`GameplayStatics.GetActorOfClass` "/Game/CJW/Blueprints/Portal/Blueprints/BP_PortalB.BP_PortalB_C"))
  (set `self.PortalB` _returnvalue))

(event `self.Box.OnComponentBeginOverlap`
  (params (OverlappedComponent :type "PrimitiveComponent Object Reference") (OtherActor :type "Actor Object Reference") (OtherComp :type "PrimitiveComponent Object Reference") (OtherBodyIndex :type Integer) (bFromSweep :type Boolean) (SweepResult :type "HitResult Structure (by ref)"))
  (`self.K2_SetActorLocationAndRotation` OtherActor (+ (`SceneComponent.K2_GetComponentLocation` (`/Game/CJW/Blueprints/Portal/Blueprints/BP_PortalB.SceneCaptureComponent2D` (`self.PortalB`))) (0.0 0.0 0.0)) (`self.K2_GetActorRotation` (`.HitActor` (`GameplayStatics.BreakHitResult` SweepResult))) false true)
  (`KismetSystemLibrary.PrintString` "Hello"))

(fn `NewFunction`
  (params (V2 :type "Vector Structure") (V1 :type "Vector Structure"))
  (returns (ReturnValue :type "Float (double-precision)"))
  (return (`KismetMathLibrary.Vector_Distance` V1 V2)))

(fn `UserConstructionScript`)