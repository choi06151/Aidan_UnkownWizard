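; BP_Item is a pickup orb that grants the player HP, score, or a bullet speed, amount or size boost when hit by the player's basic attack.
; A looping timer, gated on player status, moves the single hidden actor to a random "Item"-tagged TargetPoint.
; Each spawn picks a random type and swaps its Niagara effect.
; Timelines scale it in, then out after a delay, and hide it.
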(event `self.ReceiveBeginPlay`
  ;[1 1 1] 태어났을때 타입에따라 정해짐 ,타입에 따라 외관도 결정
  (`self.SetActorHiddenInGame` true)
  (`self.StartSetting`)
  (`KismetSystemLibrary.K2_SetTimerDelegate` (delegate `Spawn item`) 20.0 true))

(event `Spawn item`
  (bind _spawnpoint (`self.SpawnPoint`))
  ;[1 1 1] 20초마다 아이템 구슬 스폰
  (if (`|EnumEquality` (`/Game/CJW/Blueprints/Player/BP_Player.CurrentPlayerStatus` (`self.As BP Player`)) "NewEnumerator1")
    (`self.SetActorHiddenInGame` false)
    (`self.UpdateInfo`)
    (`self.K2_SetActorLocation` self (`self.K2_GetActorLocation` (`|GetArrayItem` _spawnpoint (`KismetMathLibrary.RandomInteger` (`KismetArrayLibrary.Array_Length` _spawnpoint)))) false true)
    (bind (_direction _newtrack_0) (`Timeline|Timeline` :!via `PlayFromStart`)
      (:`Update`
        (`self.SetActorScale3D` _newtrack_0)
        (`KismetSystemLibrary.Delay` 10.0)
        (`self.ReduceAppereance`)))))

(event `UpdateInfo`
  (bind _alltype (`self.AllType`))
  ;[1 1 1] 새로운아이템타입으로 변화
  (bind _output_get (set `self.CurrentItemType` (`|GetArrayItem` _alltype (`KismetMathLibrary.RandomInteger` (`KismetArrayLibrary.Array_Length` _alltype)))))
  (bind _currentappereance (`self.CurrentAppereance`)
    (:`then`
      (`ActorComponent.K2_DestroyComponent` _currentappereance)
      (switch `/Game/CJW/Blueprints/Item/EItemType` _output_get
        (:`NewEnumerator0`
          (bind _returnvalue (`NiagaraFunctionLibrary.SpawnSystemAttached` "/Game/sA_PickupSet_1/Fx/NiagaraSystems/NS_Pickup_3.NS_Pickup_3" (`self.Item`) "None" (0.0 0.0 0.0) (struct) "KeepRelativeOffset"))
          (set `self.CurrentAppereance` _returnvalue))
        (:`NewEnumerator1`
          (bind _returnvalue_2 (`NiagaraFunctionLibrary.SpawnSystemAttached` "/Game/sA_PickupSet_1/Fx/NiagaraSystems/NS_Pickup_5.NS_Pickup_5" (`self.Item`) "None" (0.0 0.0 0.0) (struct) "KeepRelativeOffset"))
          (set `self.CurrentAppereance` _returnvalue_2))
        (:`NewEnumerator2`
          (bind _returnvalue_3 (`NiagaraFunctionLibrary.SpawnSystemAttached` "/Game/sA_PickupSet_1/Fx/NiagaraSystems/NS_Pickup_2.NS_Pickup_2" (`self.Item`) "None" (0.0 0.0 0.0) (struct) "KeepRelativeOffset"))
          (set `self.CurrentAppereance` _returnvalue_3))
        (:`NewEnumerator3`
          (bind _returnvalue_4 (`NiagaraFunctionLibrary.SpawnSystemAttached` "/Game/sA_PickupSet_1/Fx/NiagaraSystems/NS_Pickup_1.NS_Pickup_1" (`self.Item`) "None" (0.0 0.0 0.0) (struct) "KeepRelativeOffset"))
          (set `self.CurrentAppereance` _returnvalue_4))
        (:`NewEnumerator4`
          (bind _returnvalue_5 (`NiagaraFunctionLibrary.SpawnSystemAttached` "/Game/sA_PickupSet_1/Fx/NiagaraSystems/NS_Pickup_4.NS_Pickup_4" (`self.Item`) "None" (0.0 0.0 0.0) (struct) "KeepRelativeOffset"))
          (set `self.CurrentAppereance` _returnvalue_5))))
    (:`else`)))

(event `ReduceAppereance`
  (bind (_direction _newtrack_0) (`Timeline|Timeline_0` :!via `PlayFromStart`)
    (:`Update`
      (`self.SetActorScale3D` _newtrack_0))
    (:`Finished`
      (`self.SetActorHiddenInGame` true))))

(event `self.Sphere.OnComponentBeginOverlap`
  (params (OverlappedComponent :type "PrimitiveComponent Object Reference") (OtherActor :type "Actor Object Reference") (OtherComp :type "PrimitiveComponent Object Reference") (OtherBodyIndex :type Integer) (bFromSweep :type Boolean) (SweepResult :type "HitResult Structure (by ref)"))
  (bind _as_bp_player (`self.As BP Player`))
  ;[1 1 1] 먹은 아이템에 종류에 따른 기능획득
  (cast `/Game/CJW/Blueprints/Bullet/BulletPool/BP_PlayerBasicAttack` OtherActor)
  (`self.SetActorHiddenInGame` true)
  (switch `/Game/CJW/Blueprints/Item/EItemType` (`self.CurrentItemType`)
    (:`NewEnumerator0`
      (`/Game/CJW/Blueprints/Player/BP_Player.GetHPItem` _as_bp_player))
    (:`NewEnumerator1`
      (`/Game/CJW/Blueprints/Player/BP_Player.GetScoreItem` _as_bp_player))
    (:`NewEnumerator2`
      (`/Game/CJW/Blueprints/Player/BP_Player.GetBulletSpeedItem` _as_bp_player))
    (:`NewEnumerator3`
      (`/Game/CJW/Blueprints/Player/BP_Player.GetBulletAmountItem` _as_bp_player))
    (:`NewEnumerator4`
      (`/Game/CJW/Blueprints/Player/BP_Player.GetBulletSizeItem` _as_bp_player))))

(fn `StartSetting`
  (bind _outactors (`GameplayStatics.GetAllActorsOfClass` "/Script/Engine.TargetPoint"))
  (for _array_element _outactors
    (if (`self.ActorHasTag` _array_element "Item")
      (`KismetArrayLibrary.Array_Add` (`self.SpawnPoint`) _array_element)))
  (bind _asbp_player (cast `/Game/CJW/Blueprints/Player/BP_Player` (`GameplayStatics.GetPlayerPawn` 0)))
  (set `self.As BP Player` _asbp_player))

(fn `UserConstructionScript`)