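; BP_SpawnUI is an actor that places itself in front of the player's camera when play begins, presumably as a UI spawn point.
; On BeginPlay it casts the first player pawn to BP_Player, stores it, then teleports itself a short fixed distance along the camera's forward vector.
; Placement happens only once; the Setlocation event is empty, and a disconnected copy of the move targets the player instead.
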(event `self.ReceiveBeginPlay`
  (bind _asbp_player (cast `/Game/CJW/Blueprints/Player/BP_Player` (`GameplayStatics.GetPlayerPawn` 0)))
  (bind _output_get (set `self.As BP Player` _asbp_player))
  (bind _camera (`/Game/CJW/Blueprints/Player/BP_Player.Camera` _output_get))
  (`self.K2_SetActorLocation` (+ (`SceneComponent.K2_GetComponentLocation` _camera) (* (`SceneComponent.GetForwardVector` _camera) 30)) false true))

(event `Set location`)

(fn `UserConstructionScript`)