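; BP_Cube is a VFX cube actor that spins and bobs up and down.
; The construction script applies a configurable mesh and scale, then creates a dynamic material instance and writes the mesh's world location into its Position parameter.
; Tick adds frame-time-scaled yaw rotation and a sine-of-game-time vertical offset, which is added per frame without delta-time scaling.
; The Position parameter is set only at construction, so it does not follow the animation.
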(event `self.ReceiveTick`
  (params (DeltaSeconds :type "Float (single-precision)"))
  (bind _cubemesh (`self.CubeMesh`))
  ;[1 1 1] Rotation and Up&Down Animation for Cube
  (`SceneComponent.K2_AddRelativeRotation` _cubemesh (`KismetMathLibrary.MakeRotator` 0.0 0.0 (* DeltaSeconds (`self.MeshRotateSpeed`))) false false)
  (`SceneComponent.K2_AddRelativeLocation` _cubemesh (`KismetMathLibrary.MakeVector` 0.0 0.0 (* (`KismetMathLibrary.Sin` (* (`GameplayStatics.GetTimeSeconds`) (`self.MeshUpDownSpeed`))) 0.4)) false false))

(fn `UserConstructionScript`
  (bind _cubemesh (`self.CubeMesh`))
  (`StaticMeshComponent.SetStaticMesh` _cubemesh (`self.SetCubeMesh`))
  (`SceneComponent.SetRelativeScale3D` _cubemesh (`self.CubeScale`))
  (bind _returnvalue (`PrimitiveComponent.CreateDynamicMaterialInstance` _cubemesh 0 (`self.CubeMaterial`) "None"))
  (bind _output_get (set `self.DynamicMaterial` _returnvalue))
  (`MaterialInstanceDynamic.SetVectorParameterValue` _output_get "Position" (`KismetMathLibrary.Conv_VectorToLinearColor` (`SceneComponent.K2_GetComponentLocation` (`self.CubeMesh`)))))