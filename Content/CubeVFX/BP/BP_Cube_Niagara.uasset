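; Cube VFX Blueprint that displays a configurable Niagara system with a continuous spin and up-and-down hover animation.
; The Construction Script assigns the chosen system to the Niagara component, resetting existing override parameters, and applies the scale variable.
; Tick adds delta-time-scaled yaw and a time-based sine Z offset to that component.
; The Z offset accumulates each frame without delta-time scaling, so bob height depends on frame rate.
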(event `self.ReceiveTick`
  (params (DeltaSeconds :type "Float (single-precision)"))
  (bind _niagara (`self.Niagara`))
  ;[1 1 1] Rotation and Up&Down Animation for Cube
  (`SceneComponent.K2_AddRelativeRotation` _niagara (`KismetMathLibrary.MakeRotator` 0.0 0.0 (* DeltaSeconds (`self.MeshRotateSpeed`))) false false)
  (`SceneComponent.K2_AddRelativeLocation` _niagara (`KismetMathLibrary.MakeVector` 0.0 0.0 (* (`KismetMathLibrary.Sin` (* (`GameplayStatics.GetTimeSeconds`) (`self.MeshUpDownSpeed`))) 0.4)) false false))

(fn `UserConstructionScript`
  (bind _niagara (`self.Niagara`))
  (`NiagaraComponent.SetAsset` _niagara (`self.SetNiagaraSystem`) true)
  (`SceneComponent.SetRelativeScale3D` _niagara (`KismetMathLibrary.Conv_DoubleToVector` (`self.NiagaraSystemScale`))))